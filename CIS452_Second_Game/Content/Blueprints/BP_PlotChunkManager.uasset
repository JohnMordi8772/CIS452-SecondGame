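; Plot chunk manager actor that expands the buildable area by spawning new BP_PlotChunk actors as existing plots fill with buildings.
; UpdateChunkCount counts plots with a valid CurrentBuilding and compares that count's share of TotalPlots to NewChunkThreshold.
; Once the threshold is reached, it spawns a chunk at the next ChunkSpawnpoints entry, in array order despite the "random" comment, until the list runs out.
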(fn `UpdateChunkCount`
  (locals (CurrentPlotCount :type "Float (double-precision)"))
  (bind _totalplots (`self.TotalPlots`))
  (bind _chunkspawnpoints (`self.ChunkSpawnpoints`))
  (bind _currentspawnpoint (`self.CurrentSpawnpoint`))
  ;[0.05937 0.05937 0.05937] Check Percent of Filled Plots
  (for _array_element _totalplots
    (if (`KismetSystemLibrary.IsValid` (`/Game/Blueprints/BuildingPlot_BP.CurrentBuilding` _array_element))
      (bind _result (`/Engine/EditorBlueprintResources/StandardMacros.IncrementFloat` (`local.CurrentPlotCount`))
        (:`  `
          (bind _returnvalue (>= (/ _result (`KismetMathLibrary.Conv_IntToDouble` (`KismetArrayLibrary.Array_Length` _totalplots))) (`self.NewChunkThreshold`)))
          (if _returnvalue
            (break))))))
  ;[0.05937 0.05937 0.05937] Pick Random Spawnpoint
  (if _returnvalue
    (if (< _currentspawnpoint (`KismetArrayLibrary.Array_Length` _chunkspawnpoints))
      (`|SpawnActorFromClass` "/Game/Blueprints/BP_PlotChunk.BP_PlotChunk_C" (`KismetMathLibrary.MakeTransform` (`|GetArrayItem` _chunkspawnpoints _currentspawnpoint)) "Undefined" "OverrideRootScale" null null)
      (`/Engine/EditorBlueprintResources/StandardMacros.IncrementInt` (`self.CurrentSpawnpoint`)))))

(fn `UserConstructionScript`)