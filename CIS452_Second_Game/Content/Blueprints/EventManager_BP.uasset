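; EventManager_BP is a timer actor that periodically refreshes city morale through CityManager_BP.
; It looks up the city manager on BeginPlay, then accumulates delta time on Tick and calls UpdateMorale every five seconds with no demolition penalty.
; A branch that would create and show the Tutorial1Event widget is unconnected and never runs.
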(event `self.ReceiveBeginPlay`
  (bind _returnvalue (`GameplayStatics.GetActorOfClass` "/Game/Blueprints/CityManager_BP.CityManager_BP_C")))

(event `self.ReceiveTick`
  (params (DeltaSeconds :type "Float (single-precision)"))
  (bind _output_get (set `self.TimePassed` (+ (`self.TimePassed`) DeltaSeconds)))
  (if (>= _output_get 5.0)
    (`/Game/Blueprints/CityManager_BP.Update Morale` (stale `self.ReceiveBeginPlay` _returnvalue) 0 false)
    (set `self.TimePassed` 0.0)))

(fn `UserConstructionScript`)