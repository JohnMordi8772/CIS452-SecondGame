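; Tutorial manager actor that presents the game's tutorial as a series of popup widgets.
; BeginPlay creates the first tutorial widget and adds it to the viewport.
; The TutorialPopupClosed event switches on an index to create and show the matching tutorial widget, with index 0 showing the first again.
; The index order departs from the widget numbering at index 4, where Tutorial7Event_2 appears before tutorials 5 to 7.
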(event `self.ReceiveBeginPlay`
  (bind _returnvalue (`|CreateWidget` "/Game/Blueprints/Events/Tutorial/Tutorial1Event.Tutorial1Event_C"))
  (`UserWidget.AddToViewport` _returnvalue 0))

(event `TutorialPopupClosed`
  (params (NewParam :type Integer))
  (switch `int` NewParam
    (:`0`
      (bind _returnvalue (`|CreateWidget` "/Game/Blueprints/Events/Tutorial/Tutorial1Event.Tutorial1Event_C"))
      (`UserWidget.AddToViewport` _returnvalue 0))
    (:`1`
      (bind _returnvalue_2 (`|CreateWidget` "/Game/Blueprints/Events/Tutorial/Tutorial2Event.Tutorial2Event_C"))
      (`UserWidget.AddToViewport` _returnvalue_2 0))
    (:`2`
      (bind _returnvalue_3 (`|CreateWidget` "/Game/Blueprints/Events/Tutorial/Tutorial3Event.Tutorial3Event_C"))
      (`UserWidget.AddToViewport` _returnvalue_3 0))
    (:`3`
      (bind _returnvalue_4 (`|CreateWidget` "/Game/Blueprints/Events/Tutorial/Tutorial4Event.Tutorial4Event_C"))
      (`UserWidget.AddToViewport` _returnvalue_4 0))
    (:`4`
      (bind _returnvalue_5 (`|CreateWidget` "/Game/Blueprints/Events/Tutorial/Tutorial7Event_2.Tutorial7Event_2_C"))
      (`UserWidget.AddToViewport` _returnvalue_5 0))
    (:`5`
      (bind _returnvalue_6 (`|CreateWidget` "/Game/Blueprints/Events/Tutorial/Tutorial5Event.Tutorial5Event_C"))
      (`UserWidget.AddToViewport` _returnvalue_6 0))
    (:`6`
      (bind _returnvalue_7 (`|CreateWidget` "/Game/Blueprints/Events/Tutorial/Tutorial6Event.Tutorial6Event_C"))
      (`UserWidget.AddToViewport` _returnvalue_7 0))
    (:`7`
      (bind _returnvalue_8 (`|CreateWidget` "/Game/Blueprints/Events/Tutorial/Tutorial7Event.Tutorial7Event_C"))
      (`UserWidget.AddToViewport` _returnvalue_8 0))))

(fn `UserConstructionScript`)