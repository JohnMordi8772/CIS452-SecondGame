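; BuildingPlot_BP is a clickable building plot that toggles a building on itself.
; Clicking destroys a valid CurrentBuilding, or spawns the placeholder TempBuildingPrefab above the plot through CreateBuilding and stores it, pending a shop menu.
; Cursor hover and clicks swap the mesh material between build and destroy previews based on occupancy, and cursor exit restores the grass material.
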(event `self.ReceiveBeginPlay`)

(event `self.ReceiveActorOnClicked`
  (params (ButtonPressed :type "Key Structure"))
  (bind _currentbuilding (`self.CurrentBuilding`))
  (bind _staticmeshcomponent (`self.StaticMeshComponent`))
  (if (`KismetSystemLibrary.IsValid` _currentbuilding)
    (`self.K2_DestroyActor` _currentbuilding)
    (else
      (bind _outbuilding (`self.CreateBuilding` (`self.TempBuildingPrefab`)))
      (set `self.CurrentBuilding` _outbuilding)))
  (if (`KismetSystemLibrary.IsValid` (`self.CurrentBuilding`)) :!label _label
    (`PrimitiveComponent.SetMaterial` _staticmeshcomponent 0 "/Game/Materials/DestroyMaterial.DestroyMaterial")
    (else
      (`PrimitiveComponent.SetMaterial` _staticmeshcomponent 0 "/Game/Materials/BuildMaterial.BuildMaterial"))))

(event `self.ReceiveActorBeginCursorOver`
  (goto _label))

(event `self.ReceiveActorEndCursorOver`
  (`PrimitiveComponent.SetMaterial` (`self.StaticMeshComponent`) 0 "/Game/StarterContent/Materials/M_Ground_Grass.M_Ground_Grass"))

(fn `CreateBuilding`
  (params (Building :type "/Game/Blueprints/BuildingBase_BP Class Reference"))
  (returns (OutBuilding :type "/Game/Blueprints/BuildingBase_BP Object Reference"))
  (bind _returnvalue (`self.GetTransform`))
  (bind _returnvalue_2 (`|SpawnActorFromClass` Building (`KismetMathLibrary.MakeTransform` (`KismetMathLibrary.MakeVector` (.x (.location _returnvalue)) (.y (.location _returnvalue)) (+ (.z (.location _returnvalue)) 100.0)) (.rotation _returnvalue) (.scale _returnvalue)) "Undefined" "OverrideRootScale" null null))
  (return _returnvalue_2))

(fn `UserConstructionScript`)