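; CityManager_BP is a city-builder manager actor that tracks morale and money income and puts the HUD_BP widget on screen at BeginPlay.
; UpdateMorale resets Morale to a base value, adds every BuildingBase_BP actor's MoraleInfluence, then subtracts a demolition penalty argument.
; UpdateMoneyRate likewise rebuilds IncreaseRate from a base rate plus each building's RateChanger.
; Both totals are recomputed by scanning all placed buildings rather than adjusted incrementally.
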(event `self.ReceiveBeginPlay`
  (bind _returnvalue (`|CreateWidget` "/Game/UI/HUD_BP.HUD_BP_C"))
  (`UserWidget.AddToViewport` _returnvalue 0))

(fn `UpdateMoneyRate`
  (bind _outactors (`GameplayStatics.GetAllActorsOfClass` "/Game/Blueprints/BuildingBase_BP.BuildingBase_BP_C"))
  (bind _output_get (set `self.IncreaseRate` (`self.BaseRate`)))
  (for _array_element _outactors
    (set `self.IncreaseRate` (+ _output_get (`/Game/Blueprints/BuildingBase_BP.RateChanger` _array_element)))))

(fn `UpdateMorale`
  (params (DemoMoraleRemoval :type Integer))
  (bind _outactors (`GameplayStatics.GetAllActorsOfClass` "/Game/Blueprints/BuildingBase_BP.BuildingBase_BP_C"))
  (bind _output_get (set `self.Morale` (`self.BaseMorale`)))
  (for _array_element _outactors
    (set `self.Morale` (+ _output_get (`/Game/Blueprints/BuildingBase_BP.Morale Influence` _array_element))))
  (set `self.Morale` (- (`self.Morale`) DemoMoraleRemoval)))

(fn `UserConstructionScript`)